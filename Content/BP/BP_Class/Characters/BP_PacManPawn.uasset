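; Player Pac-Man pawn that handles the lose condition and sound feedback; no movement logic is in its graphs.
; BeginPlay caches player pawn 0 as BP_PacManPawn and plays the Eat_ghost sound.
; Tick polls that pawn's truncated LifeCounter and, at zero, opens the lose level and plays the death sound.
; Debug key events for the four directions each play a change-direction sound.
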(event EventBeginPlay
  (bind _asbp_pac_man_pawn (Utilities|Casting|CastToBP_PacManPawn (Game|Player|GetPlayerPawn 0)))
  (Audio|SpawnSound2D "/Game/Audio/eat_ghost.eat_ghost" 1.0 1.0 0.0 0))

(event EventTick
  (params (DeltaSeconds :type Float%20%28single-precision%29))
  (switch int (Math|Float|Truncate (Variables|/Script/PacMan.PacManPawn|GetLifeCounter (stale EventBeginPlay _asbp_pac_man_pawn)))
    (:0
      (Game|OpenLevel(byObjectReference) "/Game/Levels/LoseLevel.LoseLevel")
      (Audio|SpawnSound2D "/Game/Audio/pacmandeath.pacmandeath" 1.0 1.0 0.0 0))))

(event Input|KeyboardEvents|DebugKeyUp
  (params (Key :type Key%20Structure :default "None") (ActionValue :type Input%20Action%20Value%20Structure))
  (:Pressed
    (Audio|SpawnSound2D "/Game/Audio/changedirection.changedirection" 1.0 1.0 0.0 0)))

(event Input|KeyboardEvents|DebugKeyRight
  (params (Key :type Key%20Structure :default "None") (ActionValue :type Input%20Action%20Value%20Structure))
  (:Pressed
    (Audio|SpawnSound2D "/Game/Audio/changedirection.changedirection" 1.0 1.0 0.0 0)))

(event Input|KeyboardEvents|DebugKeyLeft
  (params (Key :type Key%20Structure :default "None") (ActionValue :type Input%20Action%20Value%20Structure))
  (:Pressed
    (Audio|SpawnSound2D "/Game/Audio/changedirection.changedirection" 1.0 1.0 0.0 0)))

(event Input|KeyboardEvents|DebugKeyDown
  (params (Key :type Key%20Structure :default "None") (ActionValue :type Input%20Action%20Value%20Structure))
  (:Pressed
    (Audio|SpawnSound2D "/Game/Audio/changedirection.changedirection" 1.0 1.0 0.0 0)))

(fn ConstructionScript)

(fn NewFunction)